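; MyGameState is a GameState that runs a 60-second countdown and triggers the game-over menu when time runs out.
; SetTimer resets LeftTime and decrements it every second through a looping Delay, then calls ShowGameOver, which opens the menu on player controller 0 only.
; ClearPlayerScore zeroes the score of MyPlayerState entries in PlayerArray.
; The OnRep functions are empty, with a disconnected timer call left in one.
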(event Custom|ShowGameOver
  (bind _asmy_player_controller (Utilities|Casting|CastToMyPlayerController (Game|GetPlayerController 0)))
  (Default|ShowGameOverMenu _asmy_player_controller))

(event Custom|SetTimer
  (Variables|Default|SetLeftTime 60)
  (Utilities|FlowControl|Delay 1.0 :!label _label)
  (bind _result (Math|Integer|DecrementInt (Variables|Default|GetLeftTime))
    (:%20%20
      (if (<= _result 0)
        (CallFunction|ShowGameOver)
        (else
          (goto _label))))))

(event Custom|ClearPlayerScore
  (for _array_element (Variables|Default|GetPlayerArray self)
    (bind _asmy_player_state (Utilities|Casting|CastToMyPlayerState _array_element))
    (Variables|/Game/Blueprints/MyPlayerState.MyPlayerState_C|SetPlayerScore _asmy_player_state 0)))

(fn ConstructionScript)

(fn OnRepGameStartTimer)

(fn OnRepRandomTimerValue1)